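; Enemy rifle character that wanders between random nearby reachable points and attacks the player on sight.
; PawnSensing triggers an AI move toward the player, then fires whether the move succeeds or fails.
; Firing is throttled by a resettable DoOnce, playing a montage and damaging via a debug-drawn muzzle line trace along the mesh's right vector.
; Incoming damage lowers health, plays a hit reaction and ragdolls the mesh at zero health.
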(event OnSeePawn(PawnSensing)
  (params (Pawn :type Pawn%20Object%20Reference))
  (bind _asbp_player (Utilities|Casting|CastToBP_Player Pawn))
  (CallFunction|ChasePlayer _asbp_player))

(event Custom|Patrol
  (AI|AIMoveTo self (.RandomLocation (AI|Navigation|GetRandomReachablePointinRadius (Transformation|GetActorLocation) 3e+02 0 0)) 0 5.0 false
    (:OnSuccess
      (CallFunction|Patrol))))

(event Custom|ChasePlayer
  (params (TargetActor :type Actor%20Object%20Reference))
  (AI|AIMoveTo self "0, 0, 0" TargetActor 3e+02 false
    (:OnSuccess
      _)
    (:OnFail
      _))
  (CallFunction|Fire))

(event Custom|Fire
  (bind _rifle (Variables|Default|GetRifle))
  (bind _returnvalue (Transformation|GetSocketTransform _rifle "Muzzle" "RTS_World"))
  (Utilities|FlowControl|DoOnce false :!label _label
    (:Completed
      (Utilities|FlowControl|Sequence
        (:then_0
          (Animation|Montage|PlayMontage (Variables|Character|GetMesh) "/Game/Task_4/Animations/Fire_Rifle_Ironsights_Montage.Fire_Rifle_Ironsights_Montage"
            (:then
              (bind _outhit (Collision|LineTraceByChannel (.location _returnvalue) (+ (.location _returnvalue) (* (Math|Vector|GetRightVector (Variables|Character|GetMesh)) 3e+03)) "TraceTypeQuery1" false 0 "ForDuration"))
              (if true
                (Development|PrintString (Utilities|GetDisplayName (.HitActor (Collision|BreakHitResult _outhit))))
                (Game|Damage|ApplyDamage (.HitActor (Collision|BreakHitResult _outhit)) 2e+01 0 0)))))
        (:then_1
          (Utilities|FlowControl|Delay 0.2)
          (goto _label Reset))))))

(event Game|Damage|EventAnyDamage
  (params (Damage :type Float%20%28single-precision%29) (DamageType :type Damage%20Type%20Object%20Reference) (InstigatedBy :type Controller%20Object%20Reference) (DamageCauser :type Actor%20Object%20Reference))
  ;[0.05098 0.05098 0.05098] Take damage and animate on hit and dead
  (if (not (Variables|Default|GetIsDead))
    (Variables|Default|SetCurrentHealth (- (Variables|Default|GetCurrentHealth) Damage))
    (Animation|Montage|PlayMontage (Variables|Character|GetMesh) "/Game/Task_4/Animations/Hit_React_1_Montage.Hit_React_1_Montage"
      (:then
        (Variables|Default|SetIsDead (<= (Variables|Default|GetCurrentHealth) 0.0))
        (Development|PrintString (Utilities|String|ToString(Float) (Variables|Default|GetCurrentHealth)))
        (if (Variables|Default|GetIsDead)
          (Physics|SetSimulatePhysics (Variables|Character|GetMesh) true))))))

(event Collision|EventActorBeginOverlap
  (params (OtherActor :type Actor%20Object%20Reference)))

(event EventTick
  (params (DeltaSeconds :type Float%20%28single-precision%29)))

(event EventBeginPlay
  (Utilities|FlowControl|Delay 2.0)
  (CallFunction|Patrol))

(fn ConstructionScript)