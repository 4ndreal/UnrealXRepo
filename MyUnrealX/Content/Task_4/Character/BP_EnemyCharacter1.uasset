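; Rifle-armed enemy character that patrols random points, chases and shoots the player, and adds to the player's kill count when it dies.
; Pawn sensing triggers chase and line-trace fire through event-driven AIMoveTo calls, while a resizable sphere runs a timer that turns it toward the player.
; Damage shows a camera-facing health bar and blends physics below the hit bone for reactions, provoking a chase or ending in slow-motion ragdoll death.
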(event OnSeePawn(PawnSensing)
  (params (Pawn :type Pawn%20Object%20Reference))
  ;[0.05098 0.05098 0.05098] Enemy reaction when seeing player
  (if (not (Variables|Default|GetIsDead))
    (if (Variables|/Game/Task_4/Character/BP_Player.BP_Player_C|GetIsDead (.AsBP%20Player (Utilities|Casting|CastToBP_Player (Game|Player|GetPlayerPawn 0))))
      (CallFunction|Patrol)
      (else
        (Development|PrintString "See player")
        (Components|Sphere|SetSphereRadius (Variables|Default|GetSphere) 4e+01 true)
        (Development|PrintString "Sphere: ON" true true "(R=0.067629,G=1.000000,B=0.000000,A=1.000000)")
        (bind _asbp_player (Utilities|Casting|CastToBP_Player Pawn))
        (Utilities|FlowControl|Delay 1.0)
        (CallFunction|ChasePlayer _asbp_player)
        (CallFunction|Fire)))))

(event OnComponentBeginOverlap(Sphere)
  (params (OverlappedComponent :type Primitive%20Component%20Object%20Reference) (OtherActor :type Actor%20Object%20Reference) (OtherComp :type Primitive%20Component%20Object%20Reference) (OtherBodyIndex :type Integer) (bFromSweep :type Boolean) (SweepResult :type Hit%20Result%20Structure%20%28by%20ref%29))
  ;[0.05098 0.05098 0.05098] Sphere to make enemy look at player at certain radius
  (Development|PrintString "Player in sphere")
  (bind _asbp_player (Utilities|Casting|CastToBP_Player OtherActor))
  (Variables|Default|SetAs%20BP%20Player _asbp_player)
  (bind _returnvalue (Utilities|Time|SetTimerbyEvent (delegate Custom|Rotate) 0.01 true))
  (Variables|Default|SetTimer%20handle _returnvalue))

(event OnComponentEndOverlap(Sphere)
  (params (OverlappedComponent :type Primitive%20Component%20Object%20Reference) (OtherActor :type Actor%20Object%20Reference) (OtherComp :type Primitive%20Component%20Object%20Reference) (OtherBodyIndex :type Integer))
  ;[0.05098 0.05098 0.05098] Sphere to make enemy look at player at certain radius
  (Utilities|Time|ClearandInvalidateTimerbyHandle (Variables|Default|GetTimer%20handle))
  (Development|PrintString "Player out of Sphere "))

(event Custom|Patrol
  ;[0.05098 0.05098 0.05098] Patrol mechanism
  (if (not (Variables|Default|GetIsChasingPlayer))
    (if (not (Variables|Default|GetIsDead))
      (Development|PrintString "Patrol")
      (Components|Sphere|SetSphereRadius (Variables|Default|GetSphere) 0.0 true)
      (Development|PrintString "Sphere: OFF" true true "(R=1.000000,G=0.967155,B=0.017294,A=1.000000)")
      (Variables|/Script/Engine.CharacterMovementComponent|SetMaxWalkSpeed (Variables|Character|GetCharacterMovement) 1.5e+02)
      (AI|AIMoveTo self (.RandomLocation (AI|Navigation|GetRandomReachablePointinRadius (Transformation|GetActorLocation) 2e+03 0 0)) 0 3e+02 false
        (:OnSuccess
          (Animation|Montage|PlayMontage (Variables|Character|GetMesh) "/Game/Task_4/Animations/Idle_Rifle_Hip_Break1_Montage.Idle_Rifle_Hip_Break1_Montage"
            (:OnBlendOut
              (CallFunction|Patrol))))
        (:OnFail
          (if (not (Variables|Default|GetIsChasingPlayer))
            (CallFunction|Patrol)))))))

(event Custom|Rotate
  ;[0.05098 0.05098 0.05098] Sphere to make enemy look at player at certain radius
  (Transformation|SetActorRotation (Math|Rotator|MakeRotator 0.0 0.0 (.yaw (Math|Interpolation|RInterpTo (Transformation|GetActorRotation) (Math|Rotator|FindLookatRotation (Transformation|GetActorLocation) (Transformation|GetActorLocation (Variables|Default|GetAs%20BP%20Player))) (Utilities|Time|GetWorldDeltaSeconds) 0.93)))))

(event Custom|ChasePlayer
  (params (TargetActor :type Actor%20Object%20Reference))
  ;[0.05098 0.05098 0.05098] Chase player
  (Variables|Default|SetIsChasingPlayer true)
  (Development|PrintString "Chase player")
  (if (Variables|/Game/Task_4/Character/BP_Player.BP_Player_C|GetIsDead (.AsBP%20Player (Utilities|Casting|CastToBP_Player (Game|Player|GetPlayerPawn 0))))
    (Variables|Default|SetIsChasingPlayer false)
    (CallFunction|Patrol)
    (else
      (Variables|/Script/Engine.CharacterMovementComponent|SetMaxWalkSpeed (Variables|Character|GetCharacterMovement) 6.8e+02)
      (AI|AIMoveTo self "0, 0, 0" TargetActor 1e+03 false
        (:OnSuccess
          _)
        (:OnFail
          _))
      (Variables|/Script/Engine.CharacterMovementComponent|SetMaxWalkSpeed (Variables|Character|GetCharacterMovement) (Math|Float|Clamp(Float) 0.0 3e+02 3e+02))
      (Utilities|FlowControl|RetriggerableDelay 0.84)
      (Variables|/Script/Engine.CharacterMovementComponent|SetMaxWalkSpeed (Variables|Character|GetCharacterMovement) 6.8e+02)
      (AI|AIMoveTo self "0, 0, 0" (Game|Player|GetPlayerPawn 0) 3e+02 false
        (:then
          (Utilities|FlowControl|Delay 2.0)
          (Variables|/Script/Engine.CharacterMovementComponent|SetMaxWalkSpeed (Variables|Character|GetCharacterMovement) (Math|Float|Clamp(Float) 0.0 3e+02 3e+02))
          (AI|AIMoveTo self "0, 0, 0" (Game|Player|GetPlayerPawn 0) 1.0 false
            (:then
              (Utilities|FlowControl|Delay 1e+01)
              (Development|SetHiddeninGame (Variables|Default|GetHealthBar) true false)
              (Variables|Default|SetIsChasingPlayer false)
              (CallFunction|Patrol))))))))

(event Custom|Fire
  (bind _mesh (Variables|Character|GetMesh))
  (bind _rifle (Variables|Default|GetRifle))
  (bind _rifle_2 (Variables|Default|GetRifle))
  (bind _returnvalue (Transformation|GetSocketTransform _rifle "Muzzle" "RTS_World"))
  ;[0.05098 0.05098 0.05098] Fire mechanism
  (Variables|/Script/Engine.CharacterMovementComponent|SetMaxWalkSpeed (Variables|Character|GetCharacterMovement) (Math|Float|Clamp(Float) 0.0 3e+02 3e+02))
  (if (not (Variables|Default|GetGetDamage))
    (if (Variables|/Game/Task_4/Character/BP_Player.BP_Player_C|GetIsDead (.AsBP%20Player (Utilities|Casting|CastToBP_Player (Game|Player|GetPlayerPawn 0))))
      (CallFunction|Patrol)
      (else
        ;;[0.05098 0.05098 0.05098 1 10] If enemy is dead they stop shooting
        (if (not (Variables|Default|GetIsDead))
          (Utilities|FlowControl|DoOnce false :!label _label
            (:Completed
              (Utilities|FlowControl|Sequence
                (:then_0
                  (Animation|Montage|PlayMontage _mesh "/Game/Task_4/Animations/Fire_Rifle_Ironsights_Montage.Fire_Rifle_Ironsights_Montage"
                    (:OnBlendOut
                      (Audio|PlaySoundatLocation "/Game/StarterContent/Audio/Explosion_Cue.Explosion_Cue" (Transformation|GetActorLocation) "0, 0, 0" 2.0 1e+03 0.0 0 0 0 0)
                      (bind _outhit (Collision|LineTraceByChannel (.location _returnvalue) (+ (.location _returnvalue) (* (Math|Vector|GetRightVector _mesh) 3e+03)) "TraceTypeQuery1" false 0 "None" true "(R=0.050980,G=0.050980,B=0.050980,A=1.000000)" "(R=0.270833,G=0.012190,B=0.000000,A=1.000000)" 0.07))
                      (if true
                        (Development|PrintString (Utilities|GetDisplayName (.HitActor (Collision|BreakHitResult _outhit))))
                        (Game|Damage|ApplyDamage (.HitActor (Collision|BreakHitResult _outhit)) 2e+01 0 0)
                        (Effects|SpawnEmitterAttached "/Game/StarterContent/P_GunExplosion.P_GunExplosion" _rifle_2 "Muzzle" "10.000000,0.000000,0.000000" "0, 0, 0" "0.500000,0.500000,0.500000")
                        (Effects|SpawnEmitterAttached "/Game/InfinityBladeEffects/Effects/FX_Cines/cinema03/P_CIN_Forgemaster_ColdBreath.P_CIN_Forgemaster_ColdBreath" _rifle_2 "Muzzle" "0, 0, 0" "0, 0, 0" "2.500000,2.500000,2.500000")
                        (Effects|SpawnEmitteratLocation "/Game/InfinityBladeEffects/Effects/FX_Monsters/FX_Monster_Gruntling/Master/P_BackPack_MuzzleFlash.P_BackPack_MuzzleFlash" (.Location (Collision|BreakHitResult _outhit)) "0, 0, 0" "0.080000,0.080000,0.080000")))))
                (:then_1
                  ;;[0.05098 0.05098 0.05098] Disable movement while firing. Current status: Disabled
                  (Utilities|FlowControl|Delay 0.0)
                  (Pawn|Components|CharacterMovement|SetMovementMode (Variables|Character|GetCharacterMovement) "MOVE_Walking" 0)
                  (goto _label Reset))))))))))

(event Custom|Walk%20to%20random%20point
  ;[0.05098 0.05098 0.05098] Walk to random location
  (Variables|/Script/Engine.CharacterMovementComponent|SetMaxWalkSpeed (Variables|Character|GetCharacterMovement) (Math|Float|Clamp(Float) 0.0 3e+02 3e+02))
  (AI|AIMoveTo self (.RandomLocation (AI|Navigation|GetRandomReachablePointinRadius (Transformation|GetActorLocation) 1e+03 0 0)) 0 1.0 false
    (:OnSuccess
      (CallFunction|Patrol))))

(event Game|Damage|EventAnyDamage
  (params (Damage :type Float%20%28single-precision%29) (DamageType :type Damage%20Type%20Object%20Reference) (InstigatedBy :type Controller%20Object%20Reference) (DamageCauser :type Actor%20Object%20Reference))
  (bind _mesh (Variables|Character|GetMesh))
  (bind _hitbone (Variables|Default|GetHitBone))
  (bind _mesh_2 (Variables|Character|GetMesh))
  (bind _hitbone_2 (Variables|Default|GetHitBone))
  ;[0.05098 0.05098 0.05098] Take damage --> animate on hit and dead
  (Variables|Default|SetGetDamage true)
  (if (not (Variables|Default|GetIsDead))
    (Audio|PlaySoundatLocation "/Game/StarterContent/Audio/Voice/voice_male_d_hurt_pain_04_Cue.voice_male_d_hurt_pain_04_Cue" (Transformation|GetActorLocation) "0, 0, 0" 2.0 1.0 0.0 0 0 0 0)
    (Variables|Default|SetCurrentHealth (- (Variables|Default|GetCurrentHealth) Damage))
    (Development|PrintString "Sphere: ON" true true "(R=0.067629,G=1.000000,B=0.000000,A=1.000000)")
    (Development|SetHiddeninGame (Variables|Default|GetHealthBar) false false)
    (if (>= (Variables|Default|GetCurrentHealth) 8e+01)
      (Animation|Montage|PlayMontage (Variables|Character|GetMesh) "/Game/Task_4/Animations/Jump/Jump_From_Jog_Montage.Jump_From_Jog_Montage"
        (:OnBlendOut
          ;;[0.05098 0.05098 0.05098] Hit react blend on first time
          (Development|PrintString (Utilities|String|ToString(Name) _hitbone_2) true true "(R=0.968478,G=1.000000,B=0.957051,A=1.000000)")
          (Class|SkeletalMeshComponent|SetAllBodiesBelowSimulatePhysics _mesh _hitbone_2 true true)
          (Class|SkeletalMeshComponent|SetAllBodiesBelowPhysicsBlendWeight _mesh _hitbone_2 0.8 false true)
          (Utilities|FlowControl|Delay 0.2)
          (Class|SkeletalMeshComponent|SetAllBodiesBelowSimulatePhysics _mesh _hitbone_2 false true)
          (Transformation|AttachComponentToComponent _mesh (Variables|Collision|GetCapsuleComponent) _hitbone_2 "KeepRelative" "KeepRelative" "KeepRelative" true)
          (Transformation|SetRelativeLocationAndRotation (Variables|Character|GetMesh) "6.171243,-7.025035,-88.764606" "0.000000,270.000000,0.000000" false false))))
    (Development|PrintString (Utilities|String|Append (Utilities|GetDisplayName self) " :  " (Utilities|String|ToString(Float) (Variables|Default|GetCurrentHealth))) true true "(R=0.028941,G=0.500000,B=0.068948,A=1.000000)")
    (bind _output_get (Variables|Default|SetIsDead (<= (Variables|Default|GetCurrentHealth) 0.0)))
    (if _output_get
      (Animation|Montage|PlayMontage (Variables|Character|GetMesh) "/Game/Task_4/Animations/Jump/Jump_From_Jog_Montage.Jump_From_Jog_Montage" 1.8
        (:OnBlendOut
          (Physics|SetSimulatePhysics (Variables|Default|GetRifle) true)
          (Audio|PlaySoundatLocation "/Game/StarterContent/Audio/Voice/voice_male_d_hurt_pain_08_Cue.voice_male_d_hurt_pain_08_Cue" (Transformation|GetActorLocation) "0, 0, 0" 3.0 1.0 0.0 0 0 0 0)
          ;;[0.05098 0.05098 0.05098] Slow Motion
          (Utilities|Time|SetGlobalTimeDilation 0.5)
          (Utilities|FlowControl|Delay 0.5)
          (Utilities|Time|SetGlobalTimeDilation 1.0)
          (Collision|SetCollisionEnabled (Variables|Collision|GetCapsuleComponent) "NoCollision")
          (Development|SetHiddeninGame (Variables|Default|GetHealthBar) true false)
          (Collision|SetCollisionObjectType (Variables|Character|GetMesh) "ECC_PhysicsBody")
          ;;[0.05098 0.05098 0.05098] Scoring to Win condition
          (Utilities|FlowControl|Sequence
            (:then_0
              (bind _asbp_player (Utilities|Casting|CastToBP_Player (Game|GetPlayerCharacter 0)))
              (Math|Integer|IncrementInt (Variables|/Game/Task_4/Character/BP_Player.BP_Player_C|GetKills _asbp_player)))
            (:then_1
              (Components|DestroyComponent (Variables|Default|GetSphere))
              (Development|PrintString "Enemy deas Sphere: OFF" true true "(R=1.000000,G=0.970797,B=0.031642,A=1.000000)")))))
      (else
        ;;[0.05098 0.05098 0.05098] Hit Reaction
        (Development|PrintString (Utilities|String|ToString(Name) _hitbone) true true "(R=0.973409,G=1.000000,B=0.967060,A=1.000000)")
        (Class|SkeletalMeshComponent|SetAllBodiesBelowSimulatePhysics _mesh_2 _hitbone true true)
        (Class|SkeletalMeshComponent|SetAllBodiesBelowPhysicsBlendWeight _mesh_2 _hitbone 0.5 false true)
        (Utilities|FlowControl|Delay 0.4)
        (Class|SkeletalMeshComponent|SetAllBodiesBelowSimulatePhysics _mesh_2 _hitbone false true)
        (Transformation|AttachComponentToComponent _mesh_2 (Variables|Collision|GetCapsuleComponent) _hitbone "KeepRelative" "KeepRelative" "KeepRelative" true)
        (Transformation|SetRelativeLocationAndRotation (Variables|Character|GetMesh) "6.171243,-7.025035,-88.764606" "0.000000,270.000000,0.000000" false false)
        (Variables|Default|SetGetDamage false)
        ;;;[0.05098 0.05098 0.05098 1 10] When get hit they will chase player
        (CallFunction|ChasePlayer (Game|Player|GetPlayerPawn 0))))))

(event EventTick
  (params (DeltaSeconds :type Float%20%28single-precision%29))
  (bind _wbp_health_bar (Variables|Default|GetWBP%20Health%20Bar))
  ;[0.05098 0.05098 0.05098] Enemy HealthBar
  (Utilities|IsValid _wbp_health_bar
    (:Is%20Valid
      (Default|SetHealthbar _wbp_health_bar (Variables|Default|GetCurrentHealth) (Variables|Default|GetMaxHealth))
      (Transformation|SetWorldRotation (Variables|Default|GetHealthBar) (Math|Rotator|FindLookatRotation (Transformation|GetActorLocation) (Transformation|GetActorLocation (Game|GetPlayerCameraManager 0))) false false))))

(event EventBeginPlay
  ;[0.05098 0.05098 0.05098] Enemy HealthBar
  (bind _aswbp_health_bar (Utilities|Casting|CastToWBP_HealthBar (UserInterface|GetWidget (Variables|Default|GetHealthBar))))
  (Variables|Default|SetWBP%20Health%20Bar _aswbp_health_bar)
  (Development|SetHiddeninGame (Variables|Default|GetHealthBar) true false)
  ;;[0.05098 0.05098 0.05098] Patrol triggered
  (Utilities|FlowControl|Delay 2.0)
  (CallFunction|Patrol))

(fn ConstructionScript)

(fn SetHitBone
  (params (HitBone :type Name))
  (Variables|Default|SetHitBone HitBone))